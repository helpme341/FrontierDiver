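; BP_FrontierDiverCharacter is a diver character Blueprint that switches its movement mode to Swimming on BeginPlay.
; The rest is debug scaffolding for FrontierDiverInventoryComponent: key 2 removes the held item and prints the result, alongside a print for TakeItemToHandsByID.
; An unconnected, delayed sequence that shows and then hides the non-quick inventory widget never runs.
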(event `self.ReceiveTick`
  (params (DeltaSeconds :type "Float (single-precision)")))

(event `self.ReceiveBeginPlay`
  (`self.ChangeMovementMode` "MOVE_Swimming"))

(event `Key|One`
  (params (Key :type "Key Structure")))

(event `Key|Two`
  (params (Key :type "Key Structure"))
  (:`Pressed`
    (bind _returnvalue (`InventoryComponent.RemoveItemFromHands` (`self.FrontierDiverInventoryComponent`)))
    (`KismetSystemLibrary.PrintString` (`KismetStringLibrary.Conv_BoolToString` _returnvalue))))

(fn `UserConstructionScript`)